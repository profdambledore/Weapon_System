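; First-person player character Blueprint that handles the HUD, three-slot weapon swapping, aim down sights, reload and recoil.
; Timelines animate the active slot's component for stow and ADS, with ADS aligning the weapon's sight socket to the camera and narrowing FOV by zoom.
; A stat-scaled montage drives reloads, blocking fire until completed or cancelled.
; Recoil kicks controller input and rotates only the kinetic weapon component; recoil settling is unfinished.
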(event `self.ReceiveBeginPlay`
  (bind _returnvalue (`|CreateWidget` "/Game/Player/WBP_HUD.WBP_HUD_C"))
  (bind _output_get (set `self.HUD` _returnvalue))
  (set `/Game/Player/WBP_HUD.Player` self _output_get)
  (`UserWidget.AddToViewport` _output_get 0))

(event `InputAction|SwapPrimary`
  (params (Key :type "Key Structure"))
  ;[1 1 1] Swap Weapon
  (:`Released`
    (`self.StowCurrentWeapon` 0)))

(event `InputAction|SwapSpecial`
  (params (Key :type "Key Structure"))
  ;[1 1 1] Swap Weapon
  (:`Released`
    (`self.StowCurrentWeapon` 1)))

(event `InputAction|SwapHeavy`
  (params (Key :type "Key Structure"))
  ;[1 1 1] Swap Weapon
  (:`Released`
    (`self.StowCurrentWeapon` 2)))

(event `self.SetADSSpeed`
  (params (NewSpeed :type "Float (single-precision)"))
  ;[1 1 1] Set ADS Speed
  (`TimelineComponent.SetPlayRate` (`self.ADSTimeline`) (/ 6.0 NewSpeed)))

(event `self.AimDownSight`
  (bind (_returnvalue_location _returnvalue_rotation) (`KismetMathLibrary.BreakTransform` (`SceneComponent.GetSocketTransform` (`self.Mesh`) "GripPoint" "RTS_Actor")))
  (bind _output (`|GetArrayItem` (`self.CurrentWeapons`) (`self.CurrentWeaponIndex`)))
  (bind _returnvalue_location_2 (`KismetMathLibrary.BreakTransform` (`SceneComponent.GetSocketTransform` (`WeaponParent.Body` _output) "SightSocket" "RTS_Component")))
  ;[1 1 1] Aim Down Sight
  (if (not (`self.bInStowDraw`))
    (`/Engine/EditorBlueprintResources/StandardMacros.FlipFlop`
      (:`A`
        (set `self.bIsADS` true)
        (bind (_direction _adscurve) (`Timeline|ADSTimeline` :`NewTime` 1.0 :!label _label)
          (:`Update`
            (bind _child_actor_component (`self.GetWeaponComponent`)
              (:` `
                (bind _returnvalue (`KismetMathLibrary.RLerp` (struct) (* _returnvalue_rotation -1.0) _adscurve))
                (`SceneComponent.K2_SetRelativeLocationAndRotation` _child_actor_component (`KismetMathLibrary.VLerp` (0.0 0.0 0.0) (- (+ (- (`SceneComponent.RelativeLocation` (`self.FirstPersonCamera`)) _returnvalue_location) (20.0 0.0 0.0)) _returnvalue_location_2) _adscurve) _returnvalue false false)
                (`CameraComponent.SetFieldOfView` (`self.FirstPersonCamera`) (`KismetMathLibrary.Lerp` 90.0 (/ 90.0 (`.Zoom` (break `WeaponStats` (`WeaponParent.Stats` _output)))) _adscurve))
                (set `self.HoldLoc` _returnvalue))))))
      (:`B`
        (set `self.bIsADS` false)
        (goto _label :!via `Reverse`)))))

(event `self.VisualReload`
  (bind _output (`|GetArrayItem` (`self.CurrentWeapons`) (`self.CurrentWeaponIndex`)))
  (bind ((`Frame` _frame) (`Reload` _reload)) (break `WeaponStats` (`WeaponParent.Stats` _output)))
  ;[1 1 1] Reload
  ;;[1 1 1] Check if already in a reload
  (if (not (`self.bInReload`))
    ;;[1 1 1] Remove ability to fire
    (set `WeaponParent.bCanFire` false _output)
    (set `self.bInReload` true)
    ;;[1 1 1] Reload Timeline
    (`|PlayMontage` (`WeaponParent.Body` _output) "/Game/Weapons/AutoRifle/M_AutoRifleReload.M_AutoRifleReload" (/ (`CurveFloat.GetFloatValue` (`.Reload` (break `WeaponFrame` _frame)) _reload) 6.0)
      (:`OnCompleted`
        (`WeaponParent.RefilMagazine` _output)
        (set `self.bInReload` false :!label _label_2)
        (set `WeaponParent.bCanFire` true _output)))))

(event `self.CancelReload`
  ;[1 1 1] Reload
  ;;[1 1 1] Cancel the reload
  (`|ExecutionSequence`
    (:`then_1`
      (goto _label_2))))

(event `self.VisualRecoil`
  (params (Angle :type "Float (single-precision)") (Severity :type "Float (single-precision)"))
  (bind _kineticweaponactor (`self.KineticWeaponActor`))
  (bind (_holdloc_roll _holdloc_pitch _holdloc_yaw) (`KismetMathLibrary.BreakRotator` (`self.HoldLoc`)))
  (set `self.SettleLocation` (`SceneComponent.RelativeRotation` _kineticweaponactor))
  (`self.AddControllerYawInput` (/ Angle 10.0))
  (`self.AddControllerPitchInput` (* -1 Severity))
  ;[1 1 1] Weapon Visual Recoil
  (bind (_direction _visualrecoiltrack) (`Timeline|VisualRecoilTimeline` :!via `PlayFromStart`)
    (:`Update`
      (`SceneComponent.K2_SetRelativeRotation` _kineticweaponactor (`KismetMathLibrary.RLerp` (`KismetMathLibrary.MakeRotator` _holdloc_roll _holdloc_pitch _holdloc_yaw) (`KismetMathLibrary.MakeRotator` (+ _holdloc_roll Angle) (+ _holdloc_pitch Severity) _holdloc_yaw) _visualrecoiltrack) false false))))

(event `self.StowCurrentWeapon`
  (params (Index :type Integer))
  (if (== Index (`self.IndexSwappingTo`))
    _
    (elif (== Index (`self.CurrentWeaponIndex`))
      (if (`self.bInStowDraw`)
        (bind (_direction _stowtrack) (`Timeline|StowTimeline` :!via `Reverse` :!label _label_3)
          (:`Update`
            (bind _child_actor_component (`self.GetWeaponComponent`)
              (:` `
                (`SceneComponent.K2_SetRelativeLocation` _child_actor_component (`KismetMathLibrary.VLerp` (0.0 0.0 20.0) (0.0 0.0 -100.0) _stowtrack) false false))))
          (:`Finished`
            (`self.SwapToWeapon` Index)
            (set `self.bInStowDraw` false)
            (set `self.IndexSwappingTo` -1)
            (bind _child_actor_component_2 (`self.GetWeaponComponent`)
              (:` `
                (`SceneComponent.K2_SetRelativeLocation` _child_actor_component_2 (0.0 0.0 0.0) false false)
                (`/Game/Player/WBP_HUD.SetNewActiveWeapon` (`self.HUD`) (`self.CurrentWeaponIndex`)))))))
      (else
        (`TimelineComponent.SetPlayRate` (`self.StowTimeline`) 1.0)
        (if (`self.bIsADS`)
          (`self.AimDownSight`))
        (set `self.bInStowDraw` true)
        (set `self.IndexSwappingTo` Index)
        (`WeaponParent.StopFire` (`|GetArrayItem` (`self.CurrentWeapons`) (`self.CurrentWeaponIndex`)))
        (goto _label_3 :!via `PlayFromStart`)))))

(event `Settle`
  (if (`self.bSettled`)
    _))

(fn `UserConstructionScript`)